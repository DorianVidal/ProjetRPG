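; Chicken actor that wanders at random intervals around the location where it began play.
; A timer counted down on Tick triggers an AI MoveTo toward a random horizontal offset from that start point, drawn from separate X and Y random streams.
; The timer is parked at a large value during the move, then reset to a random delay on success or failure.
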(event Custom|MovementRandom
  (bind _newparam (CallFunction|RandomLocation))
  (AI|AIMoveTo self _newparam 0 1e+01 false
    (:then
      (Variables|Default|SetTimer 1e+04))
    (:OnSuccess
      (Variables|Default|SetTimer (Math|Random|RandomFloatinRange 5.0 1e+01) :!label _label))
    (:OnFail
      (goto _label))))

(event EventBeginPlay
  (Variables|Default|SetInitPos (Transformation|GetWorldLocation (Variables|/Script/Engine.Actor|GetRootComponent self)))
  (Variables|Default|SetTimer (Math|Random|RandomFloatinRange 5.0 1e+01)))

(event Collision|EventActorBeginOverlap
  (params (OtherActor :type Actor%20Object%20Reference)))

(event EventTick
  (params (DeltaSeconds :type Float%20%28single-precision%29))
  (Variables|Default|SetTimer (- (Variables|Default|GetTimer) DeltaSeconds))
  (if (<= (Variables|Default|GetTimer) 0.0)
    (CallFunction|MovementRandom)))

(fn ConstructionScript)

(fn RandomLocation
  (return (+ (Math|Vector|MakeVector (Math|Random|RandomFloatinRangefromStream -5e+02 5e+02 (Variables|Default|GetxRandom)) (Math|Random|RandomFloatinRangefromStream -5e+02 5e+02 (Variables|Default|GetyRandom)) 0.0) (Variables|Default|GetInitPos))))
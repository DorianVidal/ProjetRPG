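; Passage is a one-shot trigger actor that starts a dialogue approach when a ThirdPersonCharacter overlaps it.
; On overlap, it clears CanMove on player character 0, prints a French debug message, and sets ComeToDialogue on the referenced Pangolin_Blueprint.
; The IsDo flag blocks repeat triggering and is set only after the Pangolin cast succeeds.
; Nothing here restores the player's movement.
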(event EventBeginPlay)

(event Collision|EventActorBeginOverlap
  (params (OtherActor :type Actor%20Object%20Reference))
  (Utilities|Casting|CastToThirdPersonCharacter OtherActor)
  (if (Math|Boolean|Equal(Boolean) false (Variables|Default|GetIsDo))
    (bind _asthird_person_character (Utilities|Casting|CastToThirdPersonCharacter (Game|GetPlayerCharacter 0)))
    (Variables|/Game/ThirdPersonBP/Blueprints/ThirdPersonCharacter.ThirdPersonCharacter_C|SetCanMove _asthird_person_character false)
    (Development|PrintString "C'est le Joueur qui est dedans")
    (bind _aspangolin_blueprint (Utilities|Casting|CastToPangolin_Blueprint (Variables|Default|GetPangolin)))
    (Variables|/Game/Blueprints/Pangolin_Blueprint.Pangolin_Blueprint_C|SetComeToDialogue _aspangolin_blueprint true)
    (Variables|Default|SetIsDo true)))

(event EventTick
  (params (DeltaSeconds :type Float%20%28single-precision%29)))

(fn ConstructionScript)
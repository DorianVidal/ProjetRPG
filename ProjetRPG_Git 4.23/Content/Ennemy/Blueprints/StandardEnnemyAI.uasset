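; AI controller for the standard enemy, driving patrol and player detection through the StandardEnnemy_BT behavior tree.
; On BeginPlay it runs the tree, caches the controlled StandardEnnemy pawn and copies its patrol path's looping flag and wait time to the blackboard, along with a starting direction.
; AI Perception updates on the ThirdPersonCharacter write whether it was successfully sensed to the CanSeePlayer key.
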(event OnTargetPerceptionUpdated(AIPerception)
  (params (Actor :type Actor%20Object%20Reference) (Stimulus :type AI%20Stimulus%20Structure))
  (Utilities|Casting|CastToThirdPersonCharacter Actor)
  (AI|Components|Blackboard|SetValueasBool (AI|GetBlackboard 0) (Utilities|Name|MakeLiteralName "CanSeePlayer") (.bSuccessfullySensed (Utilities|Struct|BreakAIStimulus Stimulus))))

(event EventBeginPlay
  (AI|RunBehaviorTree "/Game/Ennemy/Blueprints/StandardEnnemy_BT.StandardEnnemy_BT")
  (bind _asstandard_ennemy (Utilities|Casting|CastToStandardEnnemy (Pawn|GetControlledPawn)))
  (bind _output_get (Variables|Default|SetMyPawn _asstandard_ennemy))
  (AI|Components|Blackboard|SetValueasBool (AI|GetBlackboard 0) (Utilities|Name|MakeLiteralName "PathLooping") (Variables|/Game/Ennemy/Blueprints/PatrolPath.PatrolPath_C|GetIsLooping (Variables|/Game/Ennemy/Blueprints/StandardEnnemy.StandardEnnemy_C|GetPatrolPath _output_get)))
  (Class|BlackboardComponent|SetValueasInt (AI|GetBlackboard 0) (Utilities|Name|MakeLiteralName "Direction") 1)
  (AI|Components|Blackboard|SetValueasFloat (AI|GetBlackboard 0) (Utilities|Name|MakeLiteralName "WaitTime") (Variables|/Game/Ennemy/Blueprints/PatrolPath.PatrolPath_C|GetWaitTime (Variables|/Game/Ennemy/Blueprints/StandardEnnemy.StandardEnnemy_C|GetPatrolPath (Variables|Default|GetMyPawn)))))

(fn ConstructionScript)
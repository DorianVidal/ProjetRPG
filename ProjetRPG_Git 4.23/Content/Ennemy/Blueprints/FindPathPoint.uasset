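; Behavior tree task that finds the current patrol point for a StandardEnnemy.
; It reads the path index from the blackboard, converts that PatrolPath point from the path actor's local space to world space, and writes it to the path vector key.
; The task finishes successfully only when the cast and path are valid; otherwise it never calls FinishExecute.
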(event EventReceiveExecuteAI
  (params (OwnerController :type AI%20Controller%20Object%20Reference) (ControlledPawn :type Pawn%20Object%20Reference))
  (bind _asstandard_ennemy (Utilities|Casting|CastToStandardEnnemy ControlledPawn))
  (bind _patrolpath (Variables|/Game/Ennemy/Blueprints/StandardEnnemy.StandardEnnemy_C|GetPatrolPath _asstandard_ennemy)
    (:then
      (AI|BehaviorTree|SetBlackboardValueasVector (Variables|Default|GetBB_PathVector) (Math|Transform|TransformLocation (Transformation|GetActorTransform _patrolpath) (Utilities|Array|Get(acopy) (Variables|/Game/Ennemy/Blueprints/PatrolPath.PatrolPath_C|GetPathPoints _patrolpath) (Class|BTFunctionLibrary|GetBlackboardValueasInt (Variables|Default|GetBB_PathIndex)))))
      (AI|BehaviorTree|FinishExecute true))
    (:else)))
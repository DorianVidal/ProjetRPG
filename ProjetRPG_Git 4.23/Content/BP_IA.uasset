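; BP_IA is an AI pawn that chases the player on sight or sound and can return to its starting position.
; PawnSensing sight events trigger a move toward the player; if that move fails, it waits, then heads back to the position saved at BeginPlay.
; Heard noises print their volume and trigger a move toward the player only when the player is the instigator and volume is near full.
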(event OnSeePawn(PawnSensing)
  (params (Pawn :type Pawn%20Object%20Reference))
  (Variables|Default|SetWaitAfterLost 1e+01)
  (AI|AIMoveTo self "0, 0, 0" (Game|GetPlayerCharacter 0) 1e+01 false
    (:OnFail
      (Utilities|FlowControl|Delay (Variables|Default|GetWaitAfterLost))
      (AI|AIMoveTo self (Variables|Default|GetPosInit) 0 5.0 false))))

(event OnHearNoise(PawnSensing)
  (params (Instigator :type Pawn%20Object%20Reference) (Location :type Vector%20%28by%20ref%29 :default "0, 0, 0") (Volume :type Float%20%28single-precision%29))
  (Development|PrintString (Utilities|String|ToString(Float) Volume))
  (if (== Instigator (Game|GetPlayerCharacter 0))
    (if (Math|Float|NearlyEqual(Float) Volume 1.0 0.01)
      (AI|AIMoveTo self "0, 0, 0" Instigator 5.0 false))))

(event EventBeginPlay
  (Variables|Default|SetPosInit (Transformation|GetActorLocation self)))

(event Collision|EventActorBeginOverlap
  (params (OtherActor :type Actor%20Object%20Reference)))

(event EventTick
  (params (DeltaSeconds :type Float%20%28single-precision%29)))

(fn ConstructionScript)
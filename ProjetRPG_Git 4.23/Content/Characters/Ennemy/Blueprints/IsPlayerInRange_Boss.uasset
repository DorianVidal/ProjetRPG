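; Behavior tree service for the boss enemy that starts a melee attack when the player is close.
; On activation, it compares the controlled pawn's distance to player character 0 against MeleeRange.
; Within range, it calls Attack on the BossEnnemyAI controller and sets the boss pawn's max walk speed to zero.
; The check runs only on activation, and nothing here restores the speed.
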(event EventReceiveActivationAI
  (params (OwnerController :type AI%20Controller%20Object%20Reference) (ControlledPawn :type Pawn%20Object%20Reference))
  (if (<= (Math|Float|Absolute(Float) (Transformation|GetDistanceTo ControlledPawn (Game|GetPlayerCharacter 0))) (Variables|Default|GetMeleeRange))
    (bind _asboss_ennemy_ai (Utilities|Casting|CastToBossEnnemyAI OwnerController))
    (Default|Attack _asboss_ennemy_ai)
    (Variables|/Script/Engine.CharacterMovementComponent|SetMaxWalkSpeed (Variables|/Script/Engine.Character|GetCharacterMovement (Variables|/Game/Characters/Ennemy/Boss/Blueprints/BossEnnemyAI.BossEnnemyAI_C|GetBossPawn _asboss_ennemy_ai)) 0.0)))
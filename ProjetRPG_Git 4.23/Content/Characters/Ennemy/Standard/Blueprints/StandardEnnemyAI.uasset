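; AI controller for the standard enemy, driving its patrol and player detection through the StandardEnnemy_BT behavior tree.
; On BeginPlay it caches the controlled pawn and seeds the blackboard with looping, direction and wait time, mostly from the pawn's patrol path.
; AI Perception updates set CanSeePlayer when the sensed actor is the ThirdPersonCharacter.
; An Attack event forwards to the pawn's own Attack.
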(event OnTargetPerceptionUpdated(AIPerception)
  (params (Actor :type Actor%20Object%20Reference) (Stimulus :type AI%20Stimulus%20Structure))
  (Utilities|Casting|CastToThirdPersonCharacter Actor)
  (AI|Components|Blackboard|SetValueasBool (AI|GetBlackboard 0) (Utilities|Name|MakeLiteralName "CanSeePlayer") (.bSuccessfullySensed (Utilities|Struct|BreakAIStimulus Stimulus))))

(event Custom|Attack
  (Default|Attack (Variables|Default|GetStandardEnnemyPawn)))

(event EventBeginPlay
  (AI|RunBehaviorTree "/Game/Characters/Ennemy/Standard/Blueprints/StandardEnnemy_BT.StandardEnnemy_BT")
  (bind _asstandard_ennemy (Utilities|Casting|CastToStandardEnnemy (Pawn|GetControlledPawn)))
  (bind _output_get (Variables|Default|SetStandardEnnemyPawn _asstandard_ennemy))
  (AI|Components|Blackboard|SetValueasBool (AI|GetBlackboard 0) (Utilities|Name|MakeLiteralName "PathLooping") (Variables|/Game/Characters/Ennemy/Blueprints/PatrolPath.PatrolPath_C|GetIsLooping (Variables|/Game/Characters/Ennemy/Standard/StandardEnnemy.StandardEnnemy_C|GetPatrolPath _output_get)))
  (Class|BlackboardComponent|SetValueasInt (AI|GetBlackboard 0) (Utilities|Name|MakeLiteralName "Direction") 1)
  (AI|Components|Blackboard|SetValueasFloat (AI|GetBlackboard 0) (Utilities|Name|MakeLiteralName "WaitTime") (Variables|/Game/Characters/Ennemy/Blueprints/PatrolPath.PatrolPath_C|GetWaitTime (Variables|/Game/Characters/Ennemy/Standard/StandardEnnemy.StandardEnnemy_C|GetPatrolPath (Variables|Default|GetStandardEnnemyPawn)))))

(fn ConstructionScript)
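; Behavior tree service for standard enemies that triggers an attack when the player is within melee range.
; On activation, it compares the controlled pawn's distance to the player character against MeleeRange.
; When in range, it calls Attack on the StandardEnnemyAI controller and sets the pawn's max walk speed to zero.
; The check runs only on activation, and this graph does not restore the speed.
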(event EventReceiveActivationAI
  (params (OwnerController :type AI%20Controller%20Object%20Reference) (ControlledPawn :type Pawn%20Object%20Reference))
  (if (<= (Math|Float|Absolute(Float) (Transformation|GetDistanceTo ControlledPawn (Game|GetPlayerCharacter 0))) (Variables|Default|GetMeleeRange))
    (bind _asstandard_ennemy_ai (Utilities|Casting|CastToStandardEnnemyAI OwnerController))
    (Default|Attack _asstandard_ennemy_ai)
    (Variables|/Script/Engine.CharacterMovementComponent|SetMaxWalkSpeed (Variables|/Script/Engine.Character|GetCharacterMovement (Variables|/Game/Characters/Ennemy/Standard/Blueprints/StandardEnnemyAI.StandardEnnemyAI_C|GetMyPawn _asstandard_ennemy_ai)) 0.0)))
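; BossEnnemyAI is the AI controller for the boss enemy, driving its patrol and player detection through a behavior tree.
; On BeginPlay it runs BossEnnemy_BT and seeds the blackboard with looping, direction and wait time, taking looping and wait time from the boss's patrol path.
; AI Perception updates set CanSeePlayer when the sensed actor is a ThirdPersonCharacter.
; An Attack event forwards to the controlled boss pawn's own Attack.
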(event OnTargetPerceptionUpdated(AIPerception)
  (params (Actor :type Actor%20Object%20Reference) (Stimulus :type AI%20Stimulus%20Structure))
  (Utilities|Casting|CastToThirdPersonCharacter Actor)
  (AI|Components|Blackboard|SetValueasBool (AI|GetBlackboard 0) (Utilities|Name|MakeLiteralName "CanSeePlayer") (.bSuccessfullySensed (Utilities|Struct|BreakAIStimulus Stimulus))))

(event Custom|Attack
  (Default|Attack (Variables|Default|GetBossPawn)))

(event EventBeginPlay
  (AI|RunBehaviorTree "/Game/Characters/Ennemy/Boss/Blueprints/BossEnnemy_BT.BossEnnemy_BT")
  (bind _asboss_ennemy (Utilities|Casting|CastToBossEnnemy (Pawn|GetControlledPawn)))
  (bind _output_get (Variables|Default|SetBossPawn _asboss_ennemy))
  (AI|Components|Blackboard|SetValueasBool (AI|GetBlackboard 0) (Utilities|Name|MakeLiteralName "PathLooping") (Variables|/Game/Characters/Ennemy/Blueprints/PatrolPath.PatrolPath_C|GetIsLooping (Variables|/Game/Characters/Ennemy/Boss/BossEnnemy.BossEnnemy_C|GetPatrolPath _output_get)))
  (Class|BlackboardComponent|SetValueasInt (AI|GetBlackboard 0) (Utilities|Name|MakeLiteralName "Direction") 1)
  (AI|Components|Blackboard|SetValueasFloat (AI|GetBlackboard 0) (Utilities|Name|MakeLiteralName "WaitTime") (Variables|/Game/Characters/Ennemy/Blueprints/PatrolPath.PatrolPath_C|GetWaitTime (Variables|/Game/Characters/Ennemy/Boss/BossEnnemy.BossEnnemy_C|GetPatrolPath (Variables|Default|GetBossPawn)))))

(fn ConstructionScript)
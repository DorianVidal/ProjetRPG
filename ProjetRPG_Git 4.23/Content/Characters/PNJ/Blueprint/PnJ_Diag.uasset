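; PnJ_Diag is an NPC actor that lets the player open a dialogue.
; Overlapping it shows a help TextRender and enables input from player controller 0, and leaving reverses both.
; While input is enabled, pressing F creates the PnJ_Chat widget, adds it to the viewport and shows the mouse cursor.
; The overlap events do not filter which actor triggers them.
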(event Collision|EventActorEndOverlap
  (params (OtherActor :type Actor%20Object%20Reference))
  ;[1 1 1] Affichage Aide
  (Rendering|SetVisibility (Variables|Default|GetTextRender) false false)
  (Input|DisableInput (Game|GetPlayerController 0)))

(event Collision|EventActorBeginOverlap
  (params (OtherActor :type Actor%20Object%20Reference))
  ;[1 1 1] Affichage Aide
  (Rendering|SetVisibility (Variables|Default|GetTextRender) true false)
  (Input|EnableInput (Game|GetPlayerController 0)))

(event Input|KeyboardEvents|F
  (params (Key :type Key%20Structure :default "None"))
  (bind _returnvalue (Game|GetPlayerController 0))
  ;[1 1 1] Lancement dialogue
  (:Pressed
    (bind _returnvalue_2 (UserInterface|CreateWidget "/Game/Characters/PNJ/Blueprint/PnJ_Chat.PnJ_Chat_C" _returnvalue))
    (UserInterface|Viewport|AddtoViewport _returnvalue_2 0)
    (Variables|/Script/Engine.PlayerController|SetbShowMouseCursor _returnvalue true)))

(fn ConstructionScript)
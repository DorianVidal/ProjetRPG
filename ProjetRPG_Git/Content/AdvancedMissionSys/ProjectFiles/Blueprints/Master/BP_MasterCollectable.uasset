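; Master collectable actor for the mission system, picked up when an actor implementing BPI_EventInterface overlaps its Interaction box.
; Construction fills ItemInfo with its class and self reference and configures mesh, box extent and billboard icon.
; It registers with the Objective Manager, and pickup unregisters it, reports to the Mission Manager and shows a loot notification.
; It then hides, either re-enabling and re-registering after a respawn delay or destroying itself.
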(event OnComponentBeginOverlap(Interaction)
  (params (OverlappedComponent :type Primitive%20Component%20Object%20Reference) (OtherActor :type Actor%20Object%20Reference) (OtherComp :type Primitive%20Component%20Object%20Reference) (OtherBodyIndex :type Integer) (bFromSweep :type Boolean) (SweepResult :type Hit%20Result%20Structure%20%28by%20ref%29))
  (bind _mission_events (CallFunction|GetMissionManager))
  (bind _objective (CallFunction|GetObjectiveManager))
  (bind _objective_2 (CallFunction|GetObjectiveManager))
  (bind _iteminfo (Variables|Collectable|GetItemInfo))
  (bind (_dynamicbackground_ _usematerialinstance_ _dynamicbackgroundcolor _markercolor _markericon _markericonastexture2d) (Utilities|Struct|BreakBPS_CustomMarker (.customizemarker _iteminfo)))
  (if (Utilities|DoesObjectImplementInterface OtherActor "/Game/AdvancedMissionSys/ProjectFiles/Interfaces/BPI_EventInterface.BPI_EventInterface_C")
    (Utilities|IsValid (Utilities|ToObject(Interface) _objective_2)
      (:Is%20Valid
        (Default|RemoveCollectables _objective_2 (Variables|Collectable|GetItemInfo)))
      (:Is%20Not%20Valid
        _))
    (if (Variables|Default|GetCanPickUp)
      (Variables|Default|SetCanPickUp false)
      (Collision|SetCollisionResponsetoChannel (Variables|Default|GetStaticMesh) "ECC_Pawn" "ECR_Ignore")
      (Default|CollectedItemInfo _mission_events (Variables|Collectable|GetItemInfo))
      (Default|DisplayLootNotificator _mission_events (Variables|Collectable|LootNotification|GetLootNotificationDisplayTime) (select _usematerialinstance_ _markericon _markericonastexture2d) (.name _iteminfo) (.amount _iteminfo) true "ACQUIRED" (Variables|Collectable|LootNotification|GetDynamicBackground) (Variables|Collectable|LootNotification|GetBackgroundColor) "/Game/AdvancedMissionSys/ProjectFiles/Materials/Compass/Markers/MI_MainMission.MI_MainMission")
      (Rendering|SetActorHiddenInGame true)
      (if (Variables|Collectable|GetRespawn?)
        (Utilities|FlowControl|Delay (Variables|Collectable|GetRespawnTime))
        (Rendering|SetActorHiddenInGame false)
        (Variables|Default|SetCanPickUp true)
        (Collision|SetCollisionResponsetoChannel (Variables|Default|GetInteraction) "ECC_Pawn" "ECR_Overlap")
        (Collision|SetCollisionResponsetoChannel (Variables|Default|GetStaticMesh) "ECC_Pawn" "ECR_Block")
        (Utilities|IsValid (Utilities|ToObject(Interface) _objective)
          (:Is%20Valid
            (Default|AssignCollectables _objective (Variables|Collectable|GetItemInfo))))
        (else
          (Actor|DestroyActor))))))

(event EventBeginPlay
  (Default|AssignCollectables (CallFunction|GetObjectiveManager) (Variables|Collectable|GetItemInfo)))

(event EventEndPlay
  (params (EndPlayReason :type EEndPlayReason%20Enum :default "Destroyed"))
  (bind _objective (CallFunction|GetObjectiveManager))
  (switch Utilities|FlowControl|Switch|SwitchonEEndPlayReason EndPlayReason
    (:Destroyed
      _)
    (:RemovedFromWorld
      _))
  (Utilities|IsValid (Utilities|ToObject(Interface) _objective)
    (:Is%20Valid
      (Default|RemoveCollectables _objective (Variables|Collectable|GetItemInfo)))))

(fn ConstructionScript
  (bind _interactiondistance (Variables|Collectable|GetInteractionDistance))
  (Variables|Collectable|SetItemInfo (Utilities|Struct|MakeBPS_CollectableInfo (Utilities|GetClass self) (.Name (Utilities|Struct|BreakBPS_CollectableInfo (Variables|Collectable|GetItemInfo))) (.Amount (Utilities|Struct|BreakBPS_CollectableInfo (Variables|Collectable|GetItemInfo))) (.AddMarker? (Utilities|Struct|BreakBPS_CollectableInfo (Variables|Collectable|GetItemInfo))) (.DisplayMarkerOnScreen? (Utilities|Struct|BreakBPS_CollectableInfo (Variables|Collectable|GetItemInfo))) (.MetersToAddMarker (Utilities|Struct|BreakBPS_CollectableInfo (Variables|Collectable|GetItemInfo))) (.CustomizeMarker (Utilities|Struct|BreakBPS_CollectableInfo (Variables|Collectable|GetItemInfo))) (.Mesh (Utilities|Struct|BreakBPS_CollectableInfo (Variables|Collectable|GetItemInfo))) (.ItemIcon (Utilities|Struct|BreakBPS_CollectableInfo (Variables|Collectable|GetItemInfo))) self))
  (Components|StaticMesh|SetStaticMesh (Variables|Default|GetStaticMesh) (.Mesh (Utilities|Struct|BreakBPS_CollectableInfo (Variables|Collectable|GetItemInfo))))
  (Components|Box|SetBoxExtent (Variables|Default|GetInteraction) (Math|Vector|MakeVector _interactiondistance _interactiondistance 5e+01) true)
  (Rendering|Components|Sprite|SetSprite (Variables|Default|GetBillboard) (select (== (Utilities|Struct|BreakBPS_CustomMarker (Utilities|Struct|BreakBPS_CollectableInfo (Variables|Collectable|GetItemInfo))) 0) "/Game/AdvancedMissionSys/ProjectFiles/Textures/Compass/T_Woods.T_Woods" (Utilities|Struct|BreakBPS_CustomMarker (Utilities|Struct|BreakBPS_CollectableInfo (Variables|Collectable|GetItemInfo))))))
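; Master trigger-box actor that orders an NPC to move to a target actor through the mission manager.
; The first overlap by an actor implementing BPI_EventInterface fires MoveNPCTo once, passing the NPC, target and movement, interaction and camera options.
; The construction script applies the arrow color and sizes the box from its configurable extent, with the Z extent held fixed.
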(event OnComponentBeginOverlap(Box)
  (params (OverlappedComponent :type Primitive%20Component%20Object%20Reference) (OtherActor :type Actor%20Object%20Reference) (OtherComp :type Primitive%20Component%20Object%20Reference) (OtherBodyIndex :type Integer) (bFromSweep :type Boolean) (SweepResult :type Hit%20Result%20Structure%20%28by%20ref%29))
  (if (Utilities|DoesObjectImplementInterface OtherActor "/Game/AdvancedMissionSys/ProjectFiles/Interfaces/BPI_EventInterface.BPI_EventInterface_C")
    (Utilities|FlowControl|DoOnce false
      (:Completed
        (Default|MoveNPCto (CallFunction|GetMissionManager) (Variables|MoveNPC|GetNPCToMove) (Variables|MoveNPC|GetTargetActor) (Variables|MoveNPC|GetAcceptanceRadius) (Variables|MoveNPC|GetInteractDirectly?) (Variables|MoveNPC|GetRotateCameraToNPC?) (Variables|MoveNPC|NPC|GetNPCWalkSpeed) (Variables|MoveNPC|GetStopCharacterMovement?))))))

(fn ConstructionScript
  (Components|Arrow|SetArrowColor(LinearColor) (Variables|Default|GetArrow) (Variables|MoveNPC|Defaults|GetArrowColor))
  (bind _output_get (Variables|MoveNPC|Defaults|SetCollisionBoxExtent (Math|Vector|MakeVector (.x (Variables|MoveNPC|Defaults|GetCollisionBoxExtent)) (.y (Variables|MoveNPC|Defaults|GetCollisionBoxExtent)) 1.5e+02)))
  (Components|Box|SetBoxExtent (Variables|Default|GetBox) _output_get true))
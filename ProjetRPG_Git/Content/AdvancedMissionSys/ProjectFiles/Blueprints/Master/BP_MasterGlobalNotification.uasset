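; BP_MasterGlobalNotification is a trigger actor that shows a global notification, with headline, description, XP and special-area styling, through the mission manager.
; When an actor implementing BPI_EventInterface overlaps its Box, it passes its notification properties and itself to DisplayGlobalNotification.
; The construction script sizes the Box from OverlapBoxExtent while forcing a fixed Z extent.
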(event OnComponentBeginOverlap(Box)
  (params (OverlappedComponent :type Primitive%20Component%20Object%20Reference) (OtherActor :type Actor%20Object%20Reference) (OtherComp :type Primitive%20Component%20Object%20Reference) (OtherBodyIndex :type Integer) (bFromSweep :type Boolean) (SweepResult :type Hit%20Result%20Structure%20%28by%20ref%29))
  (if (Utilities|DoesObjectImplementInterface OtherActor "/Game/AdvancedMissionSys/ProjectFiles/Interfaces/BPI_EventInterface.BPI_EventInterface_C")
    (Default|DisplayGlobalNotification (CallFunction|GetMissionManager) (Variables|GlobalNotification|GetDisplayTime) (Variables|GlobalNotification|Texts|GetHeadlineText) (Variables|GlobalNotification|Texts|GetDescription) (Variables|GlobalNotification|Bools|GetXP?) (Variables|GlobalNotification|Colors|GetXPTextColor) (Variables|GlobalNotification|GetXPValue) (Variables|GlobalNotification|Bools|GetSpecialArea?) (Variables|GlobalNotification|Texts|GetSpecialAreaText) (Variables|GlobalNotification|Colors|GetSpecialAreaBackgroundColor) self)))

(fn ConstructionScript
  (bind _output_get (Variables|GlobalNotification|SetOverlapBoxExtent (Math|Vector|MakeVector (.x (Variables|GlobalNotification|GetOverlapBoxExtent)) (.y (Variables|GlobalNotification|GetOverlapBoxExtent)) 1.5e+02)))
  (Components|Box|SetBoxExtent (Variables|Default|GetBox) _output_get true))
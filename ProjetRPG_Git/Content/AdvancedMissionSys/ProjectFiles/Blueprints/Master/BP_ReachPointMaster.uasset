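; Master reach-point actor for the mission system, marking a location that qualifying actors can reach.
; The construction script stores a self reference in ReachPointInfo and applies its arrow color and box X/Y extent, with fixed height.
; After a short BeginPlay delay it registers with the objective manager, unregistering when removed from the world.
; Box overlaps by BPI_EventInterface actors report the point's unique name to the mission manager.
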(event OnComponentBeginOverlap(Box)
  (params (OverlappedComponent :type Primitive%20Component%20Object%20Reference) (OtherActor :type Actor%20Object%20Reference) (OtherComp :type Primitive%20Component%20Object%20Reference) (OtherBodyIndex :type Integer) (bFromSweep :type Boolean) (SweepResult :type Hit%20Result%20Structure%20%28by%20ref%29))
  (if (Utilities|DoesObjectImplementInterface OtherActor "/Game/AdvancedMissionSys/ProjectFiles/Interfaces/BPI_EventInterface.BPI_EventInterface_C")
    (Default|ReachedPointInfo (CallFunction|GetMissionManager) (Utilities|Struct|BreakBPS_ReachActorInfo (Variables|ReachPointActor|GetReachPointInfo)))))

(event EventBeginPlay
  (Utilities|FlowControl|Delay 0.2)
  (Default|AssignReachPoints (CallFunction|GetObjectiveManager) (Variables|ReachPointActor|GetReachPointInfo)))

(event EventEndPlay
  (params (EndPlayReason :type EEndPlayReason%20Enum :default "Destroyed"))
  (bind _objective (CallFunction|GetObjectiveManager))
  (switch Utilities|FlowControl|Switch|SwitchonEEndPlayReason EndPlayReason
    (:RemovedFromWorld
      (Utilities|IsValid (Utilities|ToObject(Interface) _objective)
        (:Is%20Valid
          (Default|RemoveReachPoints _objective (Variables|ReachPointActor|GetReachPointInfo)))))))

(fn ConstructionScript
  (Variables|ReachPointActor|SetReachPointInfo (Utilities|Struct|MakeBPS_ReachActorInfo (.uniquename (Variables|ReachPointActor|GetReachPointInfo)) (.description (Variables|ReachPointActor|GetReachPointInfo)) (.arrowcolor (Variables|ReachPointActor|GetReachPointInfo)) (.collisionboxextent (Variables|ReachPointActor|GetReachPointInfo)) self))
  (Components|Arrow|SetArrowColor(LinearColor) (Variables|Default|GetArrow) (.arrowcolor (Variables|ReachPointActor|GetReachPointInfo)))
  (Components|Box|SetBoxExtent (Variables|Default|GetBox) (Math|Vector|MakeVector (.x (.collisionboxextent (Variables|ReachPointActor|GetReachPointInfo))) (.y (.collisionboxextent (Variables|ReachPointActor|GetReachPointInfo))) 1.5e+02) true))
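; Master enemy Blueprint for the mission system that registers with the objective manager, optionally wanders the navmesh, and tracks health.
; Death disables capsule collision and notifies the anim instance and objective manager.
; EnemyChecker overlaps pass or clear the manager's enemy reference.
; Leaving DistanceChecker, a box sized from EnemyInfo, resets a living enemy's health or starts a delayed respawn-or-destroy for a dead one, retried until the interface actor is outside.
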(event OnComponentBeginOverlap(EnemyChecker)
  (params (OverlappedComponent :type Primitive%20Component%20Object%20Reference) (OtherActor :type Actor%20Object%20Reference) (OtherComp :type Primitive%20Component%20Object%20Reference) (OtherBodyIndex :type Integer) (bFromSweep :type Boolean) (SweepResult :type Hit%20Result%20Structure%20%28by%20ref%29))
  (if (and (Utilities|DoesObjectImplementInterface OtherActor "/Game/AdvancedMissionSys/ProjectFiles/Interfaces/BPI_EventInterface.BPI_EventInterface_C") (not (Variables|Default|GetDead?)))
    (Default|PassEnemyReference (CallFunction|GetObjectiveManager) self)))

(event OnComponentEndOverlap(EnemyChecker)
  (params (OverlappedComponent :type Primitive%20Component%20Object%20Reference) (OtherActor :type Actor%20Object%20Reference) (OtherComp :type Primitive%20Component%20Object%20Reference) (OtherBodyIndex :type Integer))
  (if (Utilities|DoesObjectImplementInterface OverlappedComponent "/Game/AdvancedMissionSys/ProjectFiles/Interfaces/BPI_EventInterface.BPI_EventInterface_C")
    (Default|RemoveEnemyReference (CallFunction|GetObjectiveManager))))

(event OnComponentEndOverlap(DistanceChecker)
  (params (OverlappedComponent :type Primitive%20Component%20Object%20Reference) (OtherActor :type Actor%20Object%20Reference) (OtherComp :type Primitive%20Component%20Object%20Reference) (OtherBodyIndex :type Integer))
  (bind _enemyinfo (Variables|EnemyDefaults|GetEnemyInfo))
  (bind (_maxhealth _respawn_ _respawntime) (Utilities|Struct|BreakBPS_EnemyActorInfo _enemyinfo))
  (if (Utilities|DoesObjectImplementInterface OtherActor "/Game/AdvancedMissionSys/ProjectFiles/Interfaces/BPI_EventInterface.BPI_EventInterface_C")
    (Variables|Default|SetOutsideOfTheBox true)
    (if (Variables|Default|GetDead?)
      (if (Variables|Default|GetRespawnEnemyAfterDeath?)
        (Utilities|FlowControl|Delay _respawntime :!label _label)
        (if (Variables|Default|GetOutsideOfTheBox)
          (if _respawn_
            (Variables|Default|SetCurrentHealth _maxhealth)
            (Variables|Default|SetDead? false)
            (Class|BPIObjectivesInterface|SetEnemyasDead(Message) (Utilities|GetAnimInstance) (Utilities|Struct|BreakBPS_EnemyActorInfo (Variables|EnemyDefaults|GetEnemyInfo)) false)
            (Collision|SetCollisionEnabled (Variables|Collision|GetCapsuleComponent) "QueryAndPhysics")
            (else
              (Actor|DestroyActor)))
          (else
            (goto _label))))
      (else
        (Variables|Default|SetCurrentHealth _maxhealth)))))

(event OnComponentBeginOverlap(DistanceChecker)
  (params (OverlappedComponent :type Primitive%20Component%20Object%20Reference) (OtherActor :type Actor%20Object%20Reference) (OtherComp :type Primitive%20Component%20Object%20Reference) (OtherBodyIndex :type Integer) (bFromSweep :type Boolean) (SweepResult :type Hit%20Result%20Structure%20%28by%20ref%29))
  (if (Utilities|DoesObjectImplementInterface OtherActor "/Game/AdvancedMissionSys/ProjectFiles/Interfaces/BPI_EventInterface.BPI_EventInterface_C")
    (Variables|Default|SetOutsideOfTheBox false)))

(event Game|Damage|EventAnyDamage
  (params (Damage :type Float%20%28single-precision%29) (DamageType :type Damage%20Type%20Object%20Reference) (InstigatedBy :type Controller%20Object%20Reference) (DamageCauser :type Actor%20Object%20Reference))
  (bind _enemyinfo (Variables|EnemyDefaults|GetEnemyInfo))
  (bind _enemyuniquename (Utilities|Struct|BreakBPS_EnemyActorInfo _enemyinfo))
  (if (not (Variables|Default|GetDead?))
    (bind _output_get (Variables|Default|SetCurrentHealth (- (Variables|Default|GetCurrentHealth) Damage)))
    (if (<= _output_get 0.0)
      (Variables|Default|SetDead? true)
      (Class|BPIObjectivesInterface|SetEnemyasDead(Message) (Utilities|GetAnimInstance) _enemyuniquename true)
      (Default|SetEnemyasDead (CallFunction|GetObjectiveManager) _enemyuniquename true)
      (Collision|SetCollisionEnabled (Variables|Collision|GetCapsuleComponent) "NoCollision"))))

(event EventBeginPlay
  (Variables|Default|SetCurrentHealth (Utilities|Struct|BreakBPS_EnemyActorInfo (Variables|EnemyDefaults|GetEnemyInfo)))
  (Utilities|FlowControl|Delay 0.2)
  (Default|AssignEnemies (CallFunction|GetObjectiveManager) (Variables|EnemyDefaults|GetEnemyInfo))
  (if (and (Variables|EnemyDefaults|GetMoveToRandomLocations) (not (Variables|Default|GetDead?))) :!label _label
    (AI|AIMoveTo self (.RandomLocation (Class|NavigationSystem|GetRandomPointinNavigableRadius (Transformation|GetActorLocation self) (Variables|EnemyDefaults|GetRandomLocationRange))) 0 5.0 false
      (:OnSuccess
        (Utilities|FlowControl|Delay (Variables|EnemyDefaults|GetMoveDelay))
        (goto _label)))))

(event EventEndPlay
  (params (EndPlayReason :type EEndPlayReason%20Enum :default "Destroyed"))
  (bind _objective (CallFunction|GetObjectiveManager))
  (switch Utilities|FlowControl|Switch|SwitchonEEndPlayReason EndPlayReason
    (:RemovedFromWorld
      (Utilities|IsValid (Utilities|ToObject(Interface) _objective)
        (:Is%20Valid
          (Default|RemoveEnemies _objective (Variables|EnemyDefaults|GetEnemyInfo)))))))

(fn ConstructionScript
  (bind _output_get (Variables|EnemyDefaults|SetEnemyInfo (Utilities|Struct|MakeBPS_EnemyActorInfo (.enemyuniquename (Variables|EnemyDefaults|GetEnemyInfo)) (.maxhealth (Variables|EnemyDefaults|GetEnemyInfo)) (.respawn? (Variables|EnemyDefaults|GetEnemyInfo)) (.respawntime (Variables|EnemyDefaults|GetEnemyInfo)) (.distancetorespawn (Variables|EnemyDefaults|GetEnemyInfo)) self)))
  (Components|Box|SetBoxExtent (Variables|Default|GetDistanceChecker) (Math|Vector|MakeVector (* (Utilities|Struct|BreakBPS_EnemyActorInfo _output_get) 1e+01) (* (Utilities|Struct|BreakBPS_EnemyActorInfo _output_get) 1e+01) (* (Utilities|Struct|BreakBPS_EnemyActorInfo _output_get) 1e+01)) true))
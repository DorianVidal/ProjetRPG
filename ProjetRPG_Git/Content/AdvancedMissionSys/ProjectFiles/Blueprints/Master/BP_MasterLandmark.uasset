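; Master landmark actor for the mission system that shows itself on an actor's compass while that actor is nearby.
; Two nested box triggers form a ring: entering the outer box or leaving the inner one adds the landmark, while the opposite crossings remove it.
; Overlaps only affect actors with a BP_Mission_Component, which receives the add and remove calls.
; The construction script applies the compass icon to the billboard and sizes both boxes from variables.
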(event OnComponentBeginOverlap(BoxInner)
  (params (OverlappedComponent :type Primitive%20Component%20Object%20Reference) (OtherActor :type Actor%20Object%20Reference) (OtherComp :type Primitive%20Component%20Object%20Reference) (OtherBodyIndex :type Integer) (bFromSweep :type Boolean) (SweepResult :type Hit%20Result%20Structure%20%28by%20ref%29))
  (bind _returnvalue (Actor|GetComponentbyClass OtherActor "/Game/AdvancedMissionSys/ProjectFiles/Blueprints/Player/BP_Mission_Component.BP_Mission_Component_C"))
  (Utilities|IsValid _returnvalue
    (:Is%20Valid
      (Default|RemoveLandmarkfromCompass _returnvalue self))))

(event OnComponentEndOverlap(BoxInner)
  (params (OverlappedComponent :type Primitive%20Component%20Object%20Reference) (OtherActor :type Actor%20Object%20Reference) (OtherComp :type Primitive%20Component%20Object%20Reference) (OtherBodyIndex :type Integer))
  (bind _returnvalue (Actor|GetComponentbyClass OtherActor "/Game/AdvancedMissionSys/ProjectFiles/Blueprints/Player/BP_Mission_Component.BP_Mission_Component_C"))
  (Utilities|IsValid _returnvalue
    (:Is%20Valid
      (Default|AddLandMarktoCompass _returnvalue self))))

(event OnComponentBeginOverlap(BoxOuter)
  (params (OverlappedComponent :type Primitive%20Component%20Object%20Reference) (OtherActor :type Actor%20Object%20Reference) (OtherComp :type Primitive%20Component%20Object%20Reference) (OtherBodyIndex :type Integer) (bFromSweep :type Boolean) (SweepResult :type Hit%20Result%20Structure%20%28by%20ref%29))
  (bind _returnvalue (Actor|GetComponentbyClass OtherActor "/Game/AdvancedMissionSys/ProjectFiles/Blueprints/Player/BP_Mission_Component.BP_Mission_Component_C"))
  (Utilities|IsValid _returnvalue
    (:Is%20Valid
      (Default|AddLandMarktoCompass _returnvalue self))))

(event OnComponentEndOverlap(BoxOuter)
  (params (OverlappedComponent :type Primitive%20Component%20Object%20Reference) (OtherActor :type Actor%20Object%20Reference) (OtherComp :type Primitive%20Component%20Object%20Reference) (OtherBodyIndex :type Integer))
  (bind _returnvalue (Actor|GetComponentbyClass OtherActor "/Game/AdvancedMissionSys/ProjectFiles/Blueprints/Player/BP_Mission_Component.BP_Mission_Component_C"))
  (Utilities|IsValid _returnvalue
    (:Is%20Valid
      (Default|RemoveLandmarkfromCompass _returnvalue self))))

(fn ConstructionScript
  (Rendering|Components|Sprite|SetSprite (Variables|Default|GetBillboard) (Variables|Default|GetIconOnCompass))
  (Components|Box|SetBoxExtent (Variables|Default|GetBoxInner) (Variables|Default|GetLandmarkInnerExtent) true)
  (Components|Box|SetBoxExtent (Variables|Default|GetBoxOuter) (Variables|Default|GetLandmarkOuterExtent) true))
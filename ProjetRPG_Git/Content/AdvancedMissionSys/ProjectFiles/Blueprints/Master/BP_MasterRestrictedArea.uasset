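; BP_MasterRestrictedArea is a master Blueprint for restricted zones that drive compass highlighting through the mission system.
; Its HighlightRange box is sized from HighlightBoxExtend in the Construction Script.
; When an actor implementing BPI_EventInterface enters or leaves, it calls SpecialArea on the Mission Manager, toggling the highlight and passing compass color and text settings.
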(event OnComponentEndOverlap(HighlightRange)
  (params (OverlappedComponent :type Primitive%20Component%20Object%20Reference) (OtherActor :type Actor%20Object%20Reference) (OtherComp :type Primitive%20Component%20Object%20Reference) (OtherBodyIndex :type Integer))
  (bind _mission_events (CallFunction|GetMissionManager))
  (if (Utilities|DoesObjectImplementInterface OtherActor "/Game/AdvancedMissionSys/ProjectFiles/Interfaces/BPI_EventInterface.BPI_EventInterface_C")
    (Utilities|IsValid (Utilities|ToObject(Interface) _mission_events)
      (:Is%20Valid
        (Default|SpecialArea _mission_events (Variables|Default|GetHighlightColor) false OtherActor self (Variables|Default|GetTextOnCompass?) (Variables|Default|GetCompass%20Text) (Variables|Default|GetTextBackgroundColor))))))

(event OnComponentBeginOverlap(HighlightRange)
  (params (OverlappedComponent :type Primitive%20Component%20Object%20Reference) (OtherActor :type Actor%20Object%20Reference) (OtherComp :type Primitive%20Component%20Object%20Reference) (OtherBodyIndex :type Integer) (bFromSweep :type Boolean) (SweepResult :type Hit%20Result%20Structure%20%28by%20ref%29))
  (bind _mission_events (CallFunction|GetMissionManager))
  (if (Utilities|DoesObjectImplementInterface OtherActor "/Game/AdvancedMissionSys/ProjectFiles/Interfaces/BPI_EventInterface.BPI_EventInterface_C")
    (Utilities|IsValid (Utilities|ToObject(Interface) _mission_events)
      (:Is%20Valid
        (Default|SpecialArea _mission_events (Variables|Default|GetHighlightColor) true OtherActor self (Variables|Default|GetTextOnCompass?) (Variables|Default|GetCompass%20Text) (Variables|Default|GetTextBackgroundColor))))))

(fn ConstructionScript
  (Components|Box|SetBoxExtent (Variables|Default|GetHighlightRange) (Variables|Default|GetHighlightBoxExtend) true))
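; Player objectives component that links mission actors to BP_MasterManager and the Mission Manager, and relays enemy damage and kills.
; Assign and remove events keep the MasterManager's enemy, monster, NPC, collectable and reach point lists current as levels change.
; List edits guard against duplicates, match NPC removals by unique name, and refresh the Mission Manager after a short delay.
; It holds one current enemy reference for damage and reports kills by unique name.
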(event EventRemoveEnemies
  (params (Enemy%20To%20Remove :type BPS%20Enemy%20Actor%20Info%20Structure))
  (bind _mastermanager (Variables|Default|GetMasterManager))
  (bind _enemies (Variables|/Game/AdvancedMissionSys/ProjectFiles/Blueprints/Master/BP_MasterManager.BP_MasterManager_C|GetEnemies _mastermanager))
  ;[0 0 0 1 16] Remove Unnecessary Actor References After Level Changed
  (if (Utilities|Array|ContainsItem (Variables|/Game/AdvancedMissionSys/ProjectFiles/Blueprints/Master/BP_MasterManager.BP_MasterManager_C|GetEnemies (Variables|Default|GetMasterManager)) Enemy%20To%20Remove)
    (Utilities|Array|RemoveItem _enemies Enemy%20To%20Remove)
    (Utilities|FlowControl|Delay 0.2)
    (Default|RefreshEnemies (CallFunction|GetMissionManager) _enemies)))

(event EventAssignMonsters
  (params (Monster%20To%20Assign :type BPS%20Monster%20Info%20Structure))
  (bind _mastermanager (Variables|Default|GetMasterManager))
  (bind _monsters (Variables|/Game/AdvancedMissionSys/ProjectFiles/Blueprints/Master/BP_MasterManager.BP_MasterManager_C|GetMonsters _mastermanager))
  ;[0 0 0 1 16] Add Required Actor References After Level Changed
  (if (not (Utilities|Array|ContainsItem (Variables|/Game/AdvancedMissionSys/ProjectFiles/Blueprints/Master/BP_MasterManager.BP_MasterManager_C|GetMonsters (Variables|Default|GetMasterManager)) Monster%20To%20Assign))
    (Utilities|Array|Add _monsters Monster%20To%20Assign)
    (Utilities|FlowControl|Delay 0.2)
    (Default|RefreshMonsters (CallFunction|GetMissionManager) _monsters)))

(event EventAssignEnemies
  (params (Enemy%20To%20Assign :type BPS%20Enemy%20Actor%20Info%20Structure))
  (bind _mastermanager (Variables|Default|GetMasterManager))
  (bind _enemies (Variables|/Game/AdvancedMissionSys/ProjectFiles/Blueprints/Master/BP_MasterManager.BP_MasterManager_C|GetEnemies _mastermanager))
  ;[0 0 0 1 16] Add Required Actor References After Level Changed
  (if (not (Utilities|Array|ContainsItem (Variables|/Game/AdvancedMissionSys/ProjectFiles/Blueprints/Master/BP_MasterManager.BP_MasterManager_C|GetEnemies (Variables|Default|GetMasterManager)) Enemy%20To%20Assign))
    (Utilities|Array|Add _enemies Enemy%20To%20Assign)
    (Utilities|FlowControl|Delay 0.2)
    (Default|RefreshEnemies (CallFunction|GetMissionManager) _enemies)))

(event EventRemoveMonsters
  (params (Monster%20To%20Remove :type BPS%20Monster%20Info%20Structure))
  (bind _mastermanager (Variables|Default|GetMasterManager))
  (bind _monsters (Variables|/Game/AdvancedMissionSys/ProjectFiles/Blueprints/Master/BP_MasterManager.BP_MasterManager_C|GetMonsters _mastermanager))
  ;[0 0 0 1 16] Remove Unnecessary Actor References After Level Changed
  (if (Utilities|Array|ContainsItem (Variables|/Game/AdvancedMissionSys/ProjectFiles/Blueprints/Master/BP_MasterManager.BP_MasterManager_C|GetMonsters (Variables|Default|GetMasterManager)) Monster%20To%20Remove)
    (Utilities|Array|RemoveItem _monsters Monster%20To%20Remove)
    (Utilities|FlowControl|Delay 0.2)
    (Default|RefreshMonsters (CallFunction|GetMissionManager) _monsters)))

(event EventAssignCollectables
  (params (Collectable%20To%20Assign :type BPS%20Collectable%20Info%20Structure))
  (bind _mastermanager (Variables|Default|GetMasterManager))
  (bind _collectables (Variables|/Game/AdvancedMissionSys/ProjectFiles/Blueprints/Master/BP_MasterManager.BP_MasterManager_C|GetCollectables _mastermanager))
  ;[0 0 0 1 16] Add Required Actor References After Level Changed
  (if (not (Utilities|Array|ContainsItem (Variables|/Game/AdvancedMissionSys/ProjectFiles/Blueprints/Master/BP_MasterManager.BP_MasterManager_C|GetCollectables (Variables|Default|GetMasterManager)) Collectable%20To%20Assign))
    (Utilities|Array|Add _collectables Collectable%20To%20Assign)
    (Utilities|FlowControl|Delay 0.2)
    (Default|RefreshCollectables (CallFunction|GetMissionManager) _collectables)))

(event EventRemoveNPCs
  (params (NPC%20To%20Remove :type BPS%20NPC%20Info%20Structure))
  (bind _mastermanager (Variables|Default|GetMasterManager))
  (bind _npcs (Variables|/Game/AdvancedMissionSys/ProjectFiles/Blueprints/Master/BP_MasterManager.BP_MasterManager_C|GetNPCs _mastermanager))
  ;[0 0 0 1 16] Remove Unnecessary Actor References After Level Changed
  (for (_array_element _array_index) (Variables|/Game/AdvancedMissionSys/ProjectFiles/Blueprints/Master/BP_MasterManager.BP_MasterManager_C|GetNPCs (Variables|Default|GetMasterManager))
    (if (Utilities|Name|Equal(Name) (.MissionActorUniqueName (Utilities|Struct|BreakBPS_NPCInfo _array_element)) (.MissionActorUniqueName (Utilities|Struct|BreakBPS_NPCInfo NPC%20To%20Remove)))
      (Utilities|Array|RemoveIndex _npcs _array_index)
      (Utilities|FlowControl|Delay 0.2)
      (Default|RefreshNPCs (CallFunction|GetMissionManager) _npcs))))

(event EventRemoveCollectables
  (params (Collectable%20To%20Remove :type BPS%20Collectable%20Info%20Structure))
  (bind _mastermanager (Variables|Default|GetMasterManager))
  (bind _collectables (Variables|/Game/AdvancedMissionSys/ProjectFiles/Blueprints/Master/BP_MasterManager.BP_MasterManager_C|GetCollectables _mastermanager))
  ;[0 0 0 1 16] Remove Unnecessary Actor References After Level Changed
  (if (Utilities|Array|ContainsItem (Variables|/Game/AdvancedMissionSys/ProjectFiles/Blueprints/Master/BP_MasterManager.BP_MasterManager_C|GetCollectables (Variables|Default|GetMasterManager)) Collectable%20To%20Remove)
    (Utilities|Array|RemoveItem _collectables Collectable%20To%20Remove)
    (Utilities|FlowControl|Delay 0.2)
    (Default|RefreshCollectables (CallFunction|GetMissionManager) _collectables)))

(event EventApplyDamagetoEnemy
  (params (Damage%20To%20Apply :type Float%20%28single-precision%29))
  ;[0 0 0 1 16] Enemy/Monster Kill Events
  (Game|Damage|ApplyDamage (Variables|Default|GetEnemy) Damage%20To%20Apply 0 0))

(event EventPassEnemyReference
  (params (Enemy%20Reference :type Actor%20Object%20Reference))
  ;[0 0 0 1 16] Enemy/Monster Kill Events
  (Variables|Default|SetEnemy Enemy%20Reference))

(event EventRemoveEnemyReference
  ;[0 0 0 1 16] Enemy/Monster Kill Events
  (Variables|Default|SetEnemy 0))

(event EventSetEnemyasDead
  (params (Killed%20Enemy%20Unique%20Name :type Name :default "None") (Dead? :type Boolean))
  ;[0 0 0 1 16] Enemy/Monster Kill Events
  (Default|KilledEnemyInfo (CallFunction|GetMissionManager) Killed%20Enemy%20Unique%20Name))

(event EventAssignManagerActor
  (params (Manager%20Actor :type Actor%20Object%20Reference))
  ;[0 0 0 1 16] Assign Manager Actor
  (bind _asbp_master_manager (Utilities|Casting|CastToBP_MasterManager Manager%20Actor)
    (:then
      (Variables|Default|SetMasterManager _asbp_master_manager))
    (:CastFailed
      (Development|PrintString "Don't Forget To Add BP_MasterManager To Persistent Level!!!" true true "(R=1.000000,G=0.000000,B=0.000000,A=1.000000)" 25.0))))

(event EventAssignReachPoints
  (params (Reach%20Point%20Info%20To%20Assign :type BPS%20Reach%20Actor%20Info%20Structure))
  (bind _mastermanager (Variables|Default|GetMasterManager))
  (bind _reachpoints (Variables|/Game/AdvancedMissionSys/ProjectFiles/Blueprints/Master/BP_MasterManager.BP_MasterManager_C|GetReachPoints _mastermanager))
  ;[0 0 0 1 16] Add Required Actor References After Level Changed
  (if (not (Utilities|Array|ContainsItem (Variables|/Game/AdvancedMissionSys/ProjectFiles/Blueprints/Master/BP_MasterManager.BP_MasterManager_C|GetReachPoints (Variables|Default|GetMasterManager)) Reach%20Point%20Info%20To%20Assign))
    (Utilities|Array|Add _reachpoints Reach%20Point%20Info%20To%20Assign)
    (Utilities|FlowControl|Delay 0.2)
    (Default|RefreshReachPoints (CallFunction|GetMissionManager) _reachpoints)))

(event EventAssignNPCs
  (params (NPC%20To%20Assign :type BPS%20NPC%20Info%20Structure))
  (bind _mastermanager (Variables|Default|GetMasterManager))
  (bind _npcs (Variables|/Game/AdvancedMissionSys/ProjectFiles/Blueprints/Master/BP_MasterManager.BP_MasterManager_C|GetNPCs _mastermanager))
  ;[0 0 0 1 16] Add Required Actor References After Level Changed
  (if (not (Utilities|Array|ContainsItem (Variables|/Game/AdvancedMissionSys/ProjectFiles/Blueprints/Master/BP_MasterManager.BP_MasterManager_C|GetNPCs (Variables|Default|GetMasterManager)) NPC%20To%20Assign))
    (Utilities|Array|Add _npcs NPC%20To%20Assign)
    (Utilities|FlowControl|Delay 0.2)
    (Default|RefreshNPCs (CallFunction|GetMissionManager) _npcs)))

(event EventRemoveReachPoints
  (params (Reach%20Point%20Info%20To%20Remove :type BPS%20Reach%20Actor%20Info%20Structure))
  (bind _mastermanager (Variables|Default|GetMasterManager))
  (bind _reachpoints (Variables|/Game/AdvancedMissionSys/ProjectFiles/Blueprints/Master/BP_MasterManager.BP_MasterManager_C|GetReachPoints _mastermanager))
  ;[0 0 0 1 16] Remove Unnecessary Actor References After Level Changed
  (if (Utilities|Array|ContainsItem (Variables|/Game/AdvancedMissionSys/ProjectFiles/Blueprints/Master/BP_MasterManager.BP_MasterManager_C|GetReachPoints (Variables|Default|GetMasterManager)) Reach%20Point%20Info%20To%20Remove)
    (Utilities|Array|RemoveItem _reachpoints Reach%20Point%20Info%20To%20Remove)
    (Utilities|FlowControl|Delay 0.2)
    (Default|RefreshReachPoints (CallFunction|GetMissionManager) _reachpoints)))
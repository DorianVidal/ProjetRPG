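; BP_SideMissionActor is an example child mission actor that defines a simple side mission.
; When the last marker of mission index 0 is overlapped, it tells the Mission Manager to finish the mission as a success with a "MISSION COMPLETE" message.
; The other mission events (NPC interaction, add, start, fail, marker index) are empty hooks, and the debug index prints are unwired.
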(event EventOnMissionFailed)

(event EventOnInteractwithNPC
  (params (Interaction%20Index :type Integer)))

(event EventOnOverlappedtoLastMarker
  (params (Mission%20Index :type Integer))
  (if (== Mission%20Index 0)
    (Default|FinishMission :self (CallFunction|GetMissionManager) :Layout "NewEnumerator1" :Display%20Time 4.0 :Headline%20Text "MISSION COMPLETE" :Description%20Text "Just A Side Mission" :Reward%20Border%20Color "(R=0.356863,G=0.121569,B=0.000000,A=1.000000)" :Success? true)))

(event EventOnMissionsAdded)

(event EventGetMarkerIndex
  (params (Marker%20Index :type Integer)))

(event EventOnMissionStart)

(fn ConstructionScript
  (|CallParentFunction))